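; AI controller Blueprint for ships, holding disconnected targeting logic that currently never runs.
; Possess only calls its parent, and the NextTargetModule event is empty.
; The unwired logic picks an SB_Ship without a valid AI controller class as the owned ship's target, then starts a looping one-second timer on NextTargetModule.
; A second unwired chain steps through that target's BaseModules, setting and printing the target module.
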(event Custom|NextTargetModule)

(event EventPossess
  (params (PossessedPawn :type Pawn%20Object%20Reference))
  (|CallParentFunction PossessedPawn))

(fn ConstructionScript)